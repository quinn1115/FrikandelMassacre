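; BP_1911 is an interactable VR pistol that can be picked up, dropped and fired.
; PickUp grabs the mesh at its location with the hand's rotation through the supplied physics handle, and Drop releases it.
; Use plays the gunshot sound and muzzle flash, then runs a short debug-drawn line trace from the muzzle, whose hit result is not yet used.
; BeginPlay caches the VR player pawn.
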(event EventBeginPlay
  ;[1 1 1] Begin play
  (|CallParentFunction)
  (bind _asbp_vrplayer (Utilities|Casting|CastToBP_VRPlayer (Game|Player|GetPlayerPawn 0)))
  (Variables|Default|SetPlayer _asbp_vrplayer))

(event Collision|EventActorBeginOverlap
  (params (OtherActor :type Actor%20Object%20Reference))
  (|CallParentFunction OtherActor) ; This node is disabled and will not be called.\nDrag off pins to build functionality.
)

(event EventTick
  (params (DeltaSeconds :type Float%20%28single-precision%29))
  (|CallParentFunction DeltaSeconds) ; This node is disabled and will not be called.\nDrag off pins to build functionality.
)

(event EventPickUp
  (params (PhysicsHandle :type Physics%20Handle%20Component%20Object%20Reference) (Hand :type Grip%20Motion%20Controller%20Component%20Object%20Reference))
  (bind _mesh (Variables|Character|GetMesh))
  ;[1 1 1] Grab
  (Physics|Components|PhysicsHandle|GrabComponentatLocationwithRotation PhysicsHandle _mesh "None" (Transformation|GetWorldLocation _mesh) (Transformation|GetWorldRotation Hand)))

(event EventDrop
  (params (PhysicsHandle :type Physics%20Handle%20Component%20Object%20Reference) (Hand :type Grip%20Motion%20Controller%20Component%20Object%20Reference))
  ;[1 1 1] Drop
  (Physics|Components|PhysicsHandle|ReleaseComponent PhysicsHandle))

(event EventUse
  ;[1 1 1] Fire Weapon
  (CallFunction|FireFX)
  (CallFunction|FireLogic))

(fn ConstructionScript
  (|CallParentFunction))

(fn FireLogic
  (bind _muzzleloc (Variables|Default|GetMuzzleLoc))
  (bind _returnvalue (Transformation|GetWorldLocation _muzzleloc))
  (Collision|LineTraceByChannel _returnvalue (+ (* (Math|Vector|GetForwardVector _muzzleloc) 5e+02) _returnvalue) "TraceTypeQuery1" true 0 "ForDuration"))

(fn FireFX
  (Audio|PlaySoundatLocation (Variables|Default|GetGunShotSound) (Transformation|GetActorLocation) "0, 0, 0" 1.0 1.0 0.0 0 0 0)
  (Effects|SpawnEmitterAttached (Variables|Default|GetMuzzleFlash) (Variables|Default|GetMuzzleLoc) "None" "0, 0, 0" "0, 0, 0" "1.000000,1.000000,1.000000" "SnapToTarget"))