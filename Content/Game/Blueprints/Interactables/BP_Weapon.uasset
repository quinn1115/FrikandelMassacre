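; BP_Weapon is a grabbable shotgun interactable with VR-style reloading, held and released through a physics handle.
; Use spawns a muzzle explosion even when empty, then FireLogic spends a shell, applies recoil force and runs randomly spread line traces with debug drawing.
; Traces deal no damage and spawn fire emitters at the hit normal rather than the hit location.
; Overlapping a shell interactable with ReloadLoc destroys it and adds a shell.
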(event OnComponentBeginOverlap(ReloadLoc)
  (params (OverlappedComponent :type Primitive%20Component%20Object%20Reference) (OtherActor :type Actor%20Object%20Reference) (OtherComp :type Primitive%20Component%20Object%20Reference) (OtherBodyIndex :type Integer) (bFromSweep :type Boolean) (SweepResult :type Hit%20Result%20Structure%20%28by%20ref%29))
  ;[1 1 1] Reloading VR
  (bind _asbp_shell_interactable (Utilities|Casting|CastToBP_ShellInteractable OtherActor))
  (Actor|DestroyActor _asbp_shell_interactable)
  (Variables|Default|SetShells (+ (Variables|Default|GetShells) 1)))

(event EventBeginPlay
  (|CallParentFunction) ; This node is disabled and will not be called.\nDrag off pins to build functionality.
)

(event Collision|EventActorBeginOverlap
  (params (OtherActor :type Actor%20Object%20Reference))
  (|CallParentFunction OtherActor) ; This node is disabled and will not be called.\nDrag off pins to build functionality.
)

(event EventTick
  (params (DeltaSeconds :type Float%20%28single-precision%29))
  (|CallParentFunction DeltaSeconds) ; This node is disabled and will not be called.\nDrag off pins to build functionality.
)

(event EventPickUp
  (params (PhysicsHandle :type Physics%20Handle%20Component%20Object%20Reference) (Hand :type Grip%20Motion%20Controller%20Component%20Object%20Reference))
  (bind _returnvalue (Transformation|GetActorTransform))
  ;[1 1 1] Grab/Drop
  (Physics|Components|PhysicsHandle|GrabComponentatLocationwithRotation PhysicsHandle (Variables|Character|GetMesh) "None" (+ (.location _returnvalue) "0, 0,2.500000") (Math|Rotator|CombineRotators (.rotation _returnvalue) "45.000000, 0, 0")))

(event EventDrop
  (params (PhysicsHandle :type Physics%20Handle%20Component%20Object%20Reference) (Hand :type Grip%20Motion%20Controller%20Component%20Object%20Reference))
  ;[1 1 1] Grab/Drop
  (Physics|Components|PhysicsHandle|ReleaseComponent PhysicsHandle))

(event EventUse
  ;[1 1 1] Shotgun Shooting
  (Effects|SpawnEmitterAttached "/Game/StarterContent/Particles/P_Explosion.P_Explosion" (Variables|Default|GetMuzzle) "None" "0, 0, 0" "0, 0, 0" "1.000000,1.000000,1.000000" "SnapToTarget")
  (CallFunction|FireLogic))

(fn ConstructionScript
  (|CallParentFunction))

(fn FireLogic
  (bind _muzzle (Variables|Default|GetMuzzle))
  (bind _returnvalue (Transformation|GetWorldLocation _muzzle))
  ;[1 1 1] Shotgun Shooting
  (if (> (Variables|Default|GetShells) 0)
    (Variables|Default|SetShells (- (Variables|Default|GetShells) 1))
    (Class|PrimitiveComponent|AddForceatLocationLocal (Variables|Character|GetMesh) "-30.000000, 0, 0" "0, 0, 0" "None")
    (for _index (range 0 8)
      (bind _outhit (Collision|LineTraceByChannel _returnvalue (+ (+ (* (Math|Vector|GetForwardVector _muzzle) (Variables|Default|GetRangeShotgun)) _returnvalue) (Math|Vector|MakeVector (Math|Random|RandomFloatinRange -2e+02 2e+02) (Math|Random|RandomFloatinRange -2e+02 2e+02) (Math|Random|RandomFloatinRange -2e+02 2e+02))) "TraceTypeQuery1" false 0 "ForDuration"))
      (Effects|SpawnEmitteratLocation "/Game/StarterContent/Particles/P_Fire.P_Fire" (.Normal (Collision|BreakHitResult _outhit))))))