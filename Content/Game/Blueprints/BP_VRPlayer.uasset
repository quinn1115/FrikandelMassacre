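; VR player pawn that moves relative to the headset camera and lets each hand pick up, use and drop BP_BaseInteractable items.
; Per-hand trigger overlaps track a candidate item while that hand is free, and grab input sends it pickup or use messages.
; Items with CanUse stay held until the grip drop input, while others drop on grab release.
; Each tick, both physics handle targets follow their motion controllers.
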(event OnComponentBeginOverlap(ItemTriggerR)
  (params (OverlappedComponent :type Primitive%20Component%20Object%20Reference) (OtherActor :type Actor%20Object%20Reference) (OtherComp :type Primitive%20Component%20Object%20Reference) (OtherBodyIndex :type Integer) (bFromSweep :type Boolean) (SweepResult :type Hit%20Result%20Structure%20%28by%20ref%29))
  ;[1 1 1] Check For Near Items
  (if (not (Variables|Default|GetGrabbing_R))
    (Utilities|IsValid (Variables|Default|GetItemRight)
      (:Is%20Not%20Valid
        (bind _asbp_base_interactable (Utilities|Casting|CastToBP_BaseInteractable OtherActor))
        (Variables|Default|SetItemRight _asbp_base_interactable)))))

(event OnComponentEndOverlap(ItemTriggerL)
  (params (OverlappedComponent :type Primitive%20Component%20Object%20Reference) (OtherActor :type Actor%20Object%20Reference) (OtherComp :type Primitive%20Component%20Object%20Reference) (OtherBodyIndex :type Integer))
  ;[1 1 1] Check For Near Items
  (if (not (Variables|Default|GetGrabbing_L))
    (Utilities|Casting|CastToBP_BaseInteractable OtherActor)
    (Variables|Default|SetItemLeft 0)))

(event OnComponentBeginOverlap(ItemTriggerL)
  (params (OverlappedComponent :type Primitive%20Component%20Object%20Reference) (OtherActor :type Actor%20Object%20Reference) (OtherComp :type Primitive%20Component%20Object%20Reference) (OtherBodyIndex :type Integer) (bFromSweep :type Boolean) (SweepResult :type Hit%20Result%20Structure%20%28by%20ref%29))
  ;[1 1 1] Check For Near Items
  (if (not (Variables|Default|GetGrabbing_L))
    (Utilities|IsValid (Variables|Default|GetItemLeft)
      (:Is%20Not%20Valid
        (bind _asbp_base_interactable (Utilities|Casting|CastToBP_BaseInteractable OtherActor))
        (Variables|Default|SetItemLeft _asbp_base_interactable)))))

(event OnComponentEndOverlap(ItemTriggerR)
  (params (OverlappedComponent :type Primitive%20Component%20Object%20Reference) (OtherActor :type Actor%20Object%20Reference) (OtherComp :type Primitive%20Component%20Object%20Reference) (OtherBodyIndex :type Integer))
  ;[1 1 1] Check For Near Items
  (if (not (Variables|Default|GetGrabbing_R))
    (Utilities|Casting|CastToBP_BaseInteractable OtherActor)
    (Variables|Default|SetItemRight 0)))

(event EventBeginPlay)

(event Collision|EventActorBeginOverlap
  (params (OtherActor :type Actor%20Object%20Reference)))

(event EventTick
  (params (DeltaSeconds :type Float%20%28single-precision%29))
  (bind _leftmotioncontroller (Variables|Default|GetLeftMotionController))
  (bind _rightmotioncontroller (Variables|Default|GetRightMotionController))
  (bind _returnvalue (Transformation|GetWorldTransform _leftmotioncontroller))
  (bind _returnvalue_2 (Transformation|GetWorldTransform _rightmotioncontroller))
  ;[1 1 1] Set Target Location
  (Class|PhysicsHandleComponent|SetTargetLocationandRotation (Variables|Default|GetRMC_PH) (.location _returnvalue_2) (.rotation _returnvalue_2))
  (Class|PhysicsHandleComponent|SetTargetLocationandRotation (Variables|Default|GetLMC_PH) (.location _returnvalue) (.rotation _returnvalue)))

(event Input|ActionEvents|InputActionGrabRight
  (params (Key :type Key%20Structure))
  (bind _rmc_ph (Variables|Default|GetRMC_PH))
  (bind _rightmotioncontroller (Variables|Default|GetRightMotionController))
  ;[1 1 1] GrabRight
  (:Pressed
    (if (Variables|Default|GetGrabbing_R)
      (Class|BPIInteraction|Use(Message) (Variables|Default|GetItemRight))
      (else
        (Class|BPIInteraction|PickUp(Message) (Variables|Default|GetItemRight) _rmc_ph _rightmotioncontroller)
        (Variables|Default|SetGrabbing_R true))))
  (:Released
    (Utilities|IsValid (Variables|Default|GetItemRight)
      (:Is%20Valid
        (if (not (Variables|/Game/Game/Blueprints/Interactables/BP_BaseInteractable.BP_BaseInteractable_C|GetCanUse? (Variables|Default|GetItemRight)))
          (Class|BPIInteraction|Drop(Message) (Variables|Default|GetItemRight) _rmc_ph _rightmotioncontroller)
          (Variables|Default|SetGrabbing_R false)
          (Variables|Default|SetItemRight 0))))))

(event Input|ActionEvents|InputActionGrabLeft
  (params (Key :type Key%20Structure))
  (bind _leftmotioncontroller (Variables|Default|GetLeftMotionController))
  (bind _lmc_ph (Variables|Default|GetLMC_PH))
  ;[1 1 1] LeftHandGrab
  (:Pressed
    (if (Variables|Default|GetGrabbing_L)
      (if (Variables|/Game/Game/Blueprints/Interactables/BP_BaseInteractable.BP_BaseInteractable_C|GetCanUse? (Variables|Default|GetItemLeft))
        (Class|BPIInteraction|Use(Message) (Variables|Default|GetItemLeft)))
      (else
        (Class|BPIInteraction|PickUp(Message) (Variables|Default|GetItemLeft) _lmc_ph _leftmotioncontroller)
        (Variables|Default|SetGrabbing_L true))))
  (:Released
    (Utilities|IsValid (Variables|Default|GetItemLeft)
      (:Is%20Valid
        (if (not (Variables|/Game/Game/Blueprints/Interactables/BP_BaseInteractable.BP_BaseInteractable_C|GetCanUse? (Variables|Default|GetItemLeft)))
          (Class|BPIInteraction|Drop(Message) (Variables|Default|GetItemLeft) _lmc_ph _leftmotioncontroller)
          (Variables|Default|SetGrabbing_L false)
          (Variables|Default|SetItemLeft 0))))))

(event Input|ActionEvents|InputActionDropGripLeft
  (params (Key :type Key%20Structure))
  ;[1 1 1] Drop ByGrip
  (:Pressed
    (if (Variables|/Game/Game/Blueprints/Interactables/BP_BaseInteractable.BP_BaseInteractable_C|GetCanUse? (Variables|Default|GetItemLeft))
      (Class|BPIInteraction|Drop(Message) (Variables|Default|GetItemLeft) (Variables|Default|GetLMC_PH) (Variables|Default|GetLeftMotionController))
      (Variables|Default|SetGrabbing_L false)
      (Variables|Default|SetItemLeft 0))))

(event Input|ActionEvents|InputActionDropGripRight
  (params (Key :type Key%20Structure))
  ;[1 1 1] Drop ByGrip
  (:Pressed
    (if (Variables|/Game/Game/Blueprints/Interactables/BP_BaseInteractable.BP_BaseInteractable_C|GetCanUse? (Variables|Default|GetItemRight))
      (Class|BPIInteraction|Drop(Message) (Variables|Default|GetItemRight) (Variables|Default|GetRMC_PH) (Variables|Default|GetRightMotionController))
      (Variables|Default|SetGrabbing_R false)
      (Variables|Default|SetItemRight 0))))

(event Input|AxisEvents|InputAxisMoveForward
  (params (AxisValue :type Float%20%28single-precision%29))
  ;[1 1 1] Movement
  (Pawn|Input|AddMovementInput (Math|Vector|GetForwardVector (Variables|Default|GetVRReplicatedCamera)) AxisValue false))

(event Input|AxisEvents|InputAxisMoveRight
  (params (AxisValue :type Float%20%28single-precision%29))
  ;[1 1 1] Movement
  (Pawn|Input|AddMovementInput (Math|Vector|GetRightVector (Variables|Default|GetVRReplicatedCamera)) AxisValue false))

(fn ConstructionScript)